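; Building component for ladder pieces, adding the collision boxes for a ladder on top of its parent's collision setup.
; SpawnCollisions creates a Floor box and a Ladder box at preset transforms and extents, each with a matching debug collision.
; The Floor box blocks two custom trace channels and the Ladder box blocks a separate one.
; ReturnBoxes exposes both boxes as an array.
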(fn `ReturnBoxes`
  (returns (Boxes :type "Array of BoxComponent Object Reference"))
  (return (`|MakeArray` (`self.FloorCollision`) (`self.LadderCollision`))))

(fn `SpawnCollisions`
  (`parent.SpawnCollisions`)
  (`|ExecutionSequence`
    (:`then_0`
      ;[1 1 1] Floor
      (bind _returnvalue (`self.CreateCollision` (`self.FLOOR_LOCATION`) (`self.FLOOR_ROTATION`)))
      (bind _output_get (set `self.FloorCollision` _returnvalue))
      (`self.CreateDebugCollision` _output_get "Floor"))
    (:`then_1`
      ;[1 1 1] Ladder
      (bind _returnvalue_2 (`self.CreateCollision` (`self.LADDER_LOCATION`) (`self.LADDER_ROTATION`)))
      (bind _output_get_2 (set `self.LadderCollision` _returnvalue_2))
      (`self.CreateDebugCollision` _output_get_2 "Ladder"))
    (:`then_2`
      ;[1 1 1] Floor Default Settings
      (`BoxComponent.SetBoxExtent` (`self.FloorCollision`) (`self.FLOOR_BOX_EXTENT`) true)
      (`self.SetCollisionResponseToChannel` (`self.FloorCollision`) "ECC_GameTraceChannel6" "ECR_Block")
      (`self.SetCollisionResponseToChannel` (`self.FloorCollision`) "ECC_GameTraceChannel7" "ECR_Block"))
    (:`then_3`
      ;[1 1 1] Ladder Default Settings
      (`BoxComponent.SetBoxExtent` (`self.LadderCollision`) (`self.LADDER_BOX_EXTENT`) true)
      (`self.SetCollisionResponseToChannel` (`self.LadderCollision`) "ECC_GameTraceChannel5" "ECR_Block"))))