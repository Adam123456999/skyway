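; Building component for a triangular floor piece, adding the collision boxes along its back, left and right sides for floor and wall channels.
; SpawnCollisions runs the parent setup, then creates three floor and three wall boxes from preset transforms, each group with a shared extent and its own blocking trace channels.
; Only the wall boxes get active debug collisions; the floor debug calls are disconnected.
; ReturnBoxes exposes all six boxes.
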(fn `ReturnBoxes`
  (returns (Boxes :type "Array of BoxComponent Object Reference"))
  (return (`|MakeArray` (`self.FloorCollisionBackward`) (`self.FloorCollisionLeft`) (`self.FloorCollisionRight`) (`self.WallCollisionBackward`) (`self.WallCollisionLeft`) (`self.WallCollisionRight`))))

(fn `SpawnCollisions`
  (`parent.SpawnCollisions`)
  (`|ExecutionSequence`
    (:`then_0`
      ;[1 1 1] Floor Backward
      (bind _returnvalue (`self.CreateCollision` (`self.FLOOR_LOCATION_BACKWARD`) (`self.FLOOR_ROTATION_BACKWARD`)))
      (bind _output_get (set `self.FloorCollisionBackward` _returnvalue)))
    (:`then_1`
      ;[1 1 1] Floor Left
      (bind _returnvalue_2 (`self.CreateCollision` (`self.FLOOR_LOCATION_LEFT`) (`self.FLOOR_ROTATION_LEFT`)))
      (bind _output_get_2 (set `self.FloorCollisionLeft` _returnvalue_2)))
    (:`then_2`
      ;[1 1 1] Floor Right
      (bind _returnvalue_3 (`self.CreateCollision` (`self.FLOOR_LOCATION_RIGHT`) (`self.FLOOR_ROTATION_RIGHT`)))
      (bind _output_get_3 (set `self.FloorCollisionRight` _returnvalue_3)))
    (:`then_3`
      ;[1 1 1] Floor Default Settings
      (`BoxComponent.SetBoxExtent` (`self.FloorCollisionBackward`) (`self.FLOOR_BOX_EXTENT`) true)
      (`BoxComponent.SetBoxExtent` (`self.FloorCollisionLeft`) (`self.FLOOR_BOX_EXTENT`) true)
      (`BoxComponent.SetBoxExtent` (`self.FloorCollisionRight`) (`self.FLOOR_BOX_EXTENT`) true)
      (`self.SetCollisionResponseToChannel` (`self.FloorCollisionBackward`) "ECC_GameTraceChannel6" "ECR_Block")
      (`self.SetCollisionResponseToChannel` (`self.FloorCollisionLeft`) "ECC_GameTraceChannel6" "ECR_Block")
      (`self.SetCollisionResponseToChannel` (`self.FloorCollisionRight`) "ECC_GameTraceChannel6" "ECR_Block")
      (`self.SetCollisionResponseToChannel` (`self.FloorCollisionBackward`) "ECC_GameTraceChannel7" "ECR_Block")
      (`self.SetCollisionResponseToChannel` (`self.FloorCollisionLeft`) "ECC_GameTraceChannel7" "ECR_Block")
      (`self.SetCollisionResponseToChannel` (`self.FloorCollisionRight`) "ECC_GameTraceChannel7" "ECR_Block"))
    (:`then_4`
      ;[1 1 1] Wall Backward
      (bind _returnvalue_4 (`self.CreateCollision` (`self.WALL_LOCATION_BACKWARD`) (`self.WALL_ROTATION_BACKWARD`)))
      (bind _output_get_4 (set `self.WallCollisionBackward` _returnvalue_4))
      (`self.CreateDebugCollision` _output_get_4 "Backward"))
    (:`then_5`
      ;[1 1 1] Wall Left
      (bind _returnvalue_5 (`self.CreateCollision` (`self.WALL_LOCATION_LEFT`) (`self.WALL_ROTATION_LEFT`)))
      (bind _output_get_5 (set `self.WallCollisionLeft` _returnvalue_5))
      (`self.CreateDebugCollision` _output_get_5 "Left"))
    (:`then_6`
      ;[1 1 1] Wall Right
      (bind _returnvalue_6 (`self.CreateCollision` (`self.WALL_LOCATION_RIGHT`) (`self.WALL_ROTATION_RIGHT`)))
      (bind _output_get_6 (set `self.WallCollisionRight` _returnvalue_6))
      (`self.CreateDebugCollision` _output_get_6 "Right"))
    (:`then_7`
      ;[1 1 1] Wall Default Settings
      (`BoxComponent.SetBoxExtent` (`self.WallCollisionBackward`) (`self.WALL_BOX_EXTENT`) true)
      (`BoxComponent.SetBoxExtent` (`self.WallCollisionLeft`) (`self.WALL_BOX_EXTENT`) true)
      (`BoxComponent.SetBoxExtent` (`self.WallCollisionRight`) (`self.WALL_BOX_EXTENT`) true)
      (`self.SetCollisionResponseToChannel` (`self.WallCollisionBackward`) "ECC_GameTraceChannel4" "ECR_Block")
      (`self.SetCollisionResponseToChannel` (`self.WallCollisionLeft`) "ECC_GameTraceChannel4" "ECR_Block")
      (`self.SetCollisionResponseToChannel` (`self.WallCollisionRight`) "ECC_GameTraceChannel4" "ECR_Block"))))