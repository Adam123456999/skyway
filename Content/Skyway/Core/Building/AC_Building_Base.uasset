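; AC_Building_Base is a base component for building collision on its owner, with a helper that casts that owner to BP_Ship_Base.
; BeginPlay calls SpawnCollisions, an empty stub like GetHit and ReturnBoxes, presumably for children to override.
; CreateCollision adds boxes at owner-relative offsets, while CreateDebugCollision optionally attaches an arrow and direction label.
; EndPlay sends the owner a DestroyBuildingMessage for each returned box.
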(event `self.ReceiveBeginPlay`
  (`self.SpawnCollisions`))

(event `self.ReceiveEndPlay`
  (params (EndPlayReason :type "EEndPlayReason Enum" :default "Destroyed"))
  (bind _boxes (`self.ReturnBoxes`))
  (for _array_element _boxes
    (message `/Game/Skyway/Core/Ship/BPI_Ship.DestroyBuilding` (`self.GetOwner`) _array_element)))

(fn `CalculateWorldLocation`
  (params (RelativeLocation :type "Vector Structure"))
  (returns (ReturnValue :type "Vector Structure"))
  (bind _returnvalue (`self.GetOwner`))
  (return (+ (`Actor.K2_GetActorLocation` _returnvalue) (* (`Actor.GetActorForwardVector` _returnvalue) (.x (`local.RelativeLocation`))) (* (`Actor.GetActorRightVector` _returnvalue) (.y (`local.RelativeLocation`))) (* (`Actor.GetActorUpVector` _returnvalue) (.z (`local.RelativeLocation`))))))

(fn `CreateCollision`
  (params (`Relative Location` :type "Vector Structure") (RelativeRotation :type "Rotator Structure"))
  (returns (ReturnValue :type "BoxComponent Object Reference"))
  (locals (L_BoxCollision :type "BoxComponent Object Reference"))
  (bind _returnvalue (`|AddComponentByClass` (`self.GetOwner`) "/Script/Engine.BoxComponent" false (`/Game/Skyway/Core/Engine/MLBP_Defaults.DEFAULT`)))
  (bind _output_get (set `local.L_BoxCollision` _returnvalue))
  (`self.K2_AttachToComponent` _output_get self "None" "KeepRelative" "KeepRelative" "KeepRelative" true)
  (`self.K2_SetWorldLocation` (`local.L_BoxCollision`) (`self.CalculateWorldLocation` (`local.Relative Location`)) false false)
  (`self.K2_SetRelativeRotation` (`local.L_BoxCollision`) (`local.RelativeRotation`) false false)
  (return (`local.L_BoxCollision`)))

(fn `CreateDebugCollision`
  (params (Collision :type "BoxComponent Object Reference") (CollisionDirection :type Text))
  (locals (L_DebugArrow :type "ArrowComponent Object Reference") (L_DebugText :type "TextRenderComponent Object Reference"))
  (bind _returnvalue (`/Game/Skyway/Core/Engine/FLBP_Defaults.GetDebugUseCase`))
  (if _returnvalue
    (bind _returnvalue_2 (`|AddComponentByClass` (`self.GetOwner`) "/Script/Engine.ArrowComponent" false (`/Game/Skyway/Core/Engine/MLBP_Defaults.DEFAULT`)))
    (bind _output_get (set `local.L_DebugArrow` _returnvalue_2))
    (`self.K2_AttachToComponent` _output_get (`local.Collision`) "None" "KeepRelative" "KeepRelative" "KeepRelative" true)
    (`self.SetHiddenInGame` (`local.L_DebugArrow`) false false)
    (bind _returnvalue_3 (`|AddComponentByClass` (`self.GetOwner`) "/Script/Engine.TextRenderComponent" false (`/Game/Skyway/Core/Engine/MLBP_Defaults.DEFAULT`)))
    (bind _output_get_2 (set `local.L_DebugText` _returnvalue_3))
    (`self.K2_AttachToComponent` _output_get_2 (`local.Collision`) "None" "KeepRelative" "KeepRelative" "KeepRelative" true)
    (`TextRenderComponent.SetTextRenderColor` :`self` (`local.L_DebugText`))
    (`TextRenderComponent.K2_SetText` (`local.L_DebugText`) (`local.CollisionDirection`))))

(fn `GetHit`
  (returns (HitMesh :type Boolean))
  (return false))

(fn `GetShip`
  (returns (ReturnValue :type "/Game/Skyway/Core/Ship/BP_Ship_Base Object Reference"))
  (bind _asbp_ship_base (cast `/Game/Skyway/Core/Ship/BP_Ship_Base` (`self.GetOwner`)))
  (return _asbp_ship_base))

(fn `ReturnBoxes`
  (returns (Boxes :type "Array of BoxComponent Object Reference"))
  (return))

(fn `SpawnCollisions`)