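; AC_Building_Wall is a building component for wall pieces that creates box collisions for the wall itself and for floor positions to its left and right.
; SpawnCollisions runs the parent logic, then creates each box at a preset transform with a direction-labeled debug collision.
; It then sizes the boxes and sets separate custom trace channels to Block for wall and floor boxes.
; ReturnBoxes exposes all three boxes as an array.
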(fn `ReturnBoxes`
  (returns (Boxes :type "Array of BoxComponent Object Reference"))
  (return (`|MakeArray` (`self.WallCollision`) (`self.FloorCollisionLeft`) (`self.FloorCollisionRight`))))

(fn `SpawnCollisions`
  (`parent.SpawnCollisions`)
  (`|ExecutionSequence`
    (:`then_0`
      ;[1 1 1] Wall
      (bind _returnvalue (`self.CreateCollision` (`self.WALL_LOCATION`) (`self.WALL_ROTATION`)))
      (bind _output_get (set `self.WallCollision` _returnvalue))
      (`self.CreateDebugCollision` _output_get "Forward"))
    (:`then_1`
      ;[1 1 1] Floor Left
      (bind _returnvalue_2 (`self.CreateCollision` (`self.FLOOR_LOCATION_LEFT`) (`self.FLOOR_ROTATION_LEFT`)))
      (bind _output_get_2 (set `self.FloorCollisionLeft` _returnvalue_2))
      (`self.CreateDebugCollision` _output_get_2 "Left"))
    (:`then_2`
      ;[1 1 1] Floor Right
      (bind _returnvalue_3 (`self.CreateCollision` (`self.FLOOR_LOCATION_RIGHT`) (`self.FLOOR_ROTATION_RIGHT`)))
      (bind _output_get_3 (set `self.FloorCollisionRight` _returnvalue_3))
      (`self.CreateDebugCollision` _output_get_3 "Right"))
    (:`then_3`
      ;[1 1 1] Collision Default Settings
      (`BoxComponent.SetBoxExtent` (`self.WallCollision`) (`self.WALL_BOX_EXTENT`) true)
      (`BoxComponent.SetBoxExtent` (`self.FloorCollisionLeft`) (`self.FLOOR_BOX_EXTENT`) true)
      (`BoxComponent.SetBoxExtent` (`self.FloorCollisionRight`) (`self.FLOOR_BOX_EXTENT`) true)
      (`self.SetCollisionResponseToChannel` (`self.WallCollision`) "ECC_GameTraceChannel4" "ECR_Block")
      (`self.SetCollisionResponseToChannel` (`self.FloorCollisionLeft`) "ECC_GameTraceChannel6" "ECR_Block")
      (`self.SetCollisionResponseToChannel` (`self.FloorCollisionRight`) "ECC_GameTraceChannel6" "ECR_Block")
      (`self.SetCollisionResponseToChannel` (`self.FloorCollisionLeft`) "ECC_GameTraceChannel7" "ECR_Block")
      (`self.SetCollisionResponseToChannel` (`self.FloorCollisionRight`) "ECC_GameTraceChannel7" "ECR_Block"))))