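; Floor building component that creates the collision boxes around a floor piece, likely as snap targets for placing adjacent pieces.
; SpawnCollisions extends the parent to create four directional floor boxes, four wall boxes and a ladder box at preset transforms and extents.
; Each group blocks its own custom trace channels, some boxes also get debug collisions, and ReturnBoxes returns all nine.
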(fn `ReturnBoxes`
  (returns (Boxes :type "Array of BoxComponent Object Reference"))
  (return (`|MakeArray` (`self.FloorCollisionForward`) (`self.FloorCollisionBackward`) (`self.FloorCollisionLeft`) (`self.FloorCollisionRight`) (`self.WallCollisionForward`) (`self.WallCollisionBackward`) (`self.WallCollisionLeft`) (`self.WallCollisionRight`) (`self.LadderCollision`))))

(fn `SpawnCollisions`
  (`parent.SpawnCollisions`)
  (`|ExecutionSequence`
    (:`then_0`
      ;[1 1 1] Floor Forward
      (bind _returnvalue (`self.CreateCollision` (`self.FLOOR_LOCATION_FORWARD`) (`self.FLOOR_ROTATION_FORWARD`)))
      (bind _output_get (set `self.FloorCollisionForward` _returnvalue))
      (`self.CreateDebugCollision` _output_get "Forward"))
    (:`then_1`
      ;[1 1 1] Floor Backward
      (bind _returnvalue_2 (`self.CreateCollision` (`self.FLOOR_LOCATION_BACKWARD`) (`self.FLOOR_ROTATION_BACKWARD`)))
      (bind _output_get_2 (set `self.FloorCollisionBackward` _returnvalue_2)))
    (:`then_2`
      ;[1 1 1] Floor Left
      (bind _returnvalue_3 (`self.CreateCollision` (`self.FLOOR_LOCATION_LEFT`) (`self.FLOOR_ROTATION_LEFT`)))
      (bind _output_get_3 (set `self.FloorCollisionLeft` _returnvalue_3)))
    (:`then_3`
      ;[1 1 1] Floor Right
      (bind _returnvalue_4 (`self.CreateCollision` (`self.FLOOR_LOCATION_RIGHT`) (`self.FLOOR_ROTATION_RIGHT`)))
      (bind _output_get_4 (set `self.FloorCollisionRight` _returnvalue_4)))
    (:`then_4`
      ;[1 1 1] Floor Default Settings
      (`BoxComponent.SetBoxExtent` (`self.FloorCollisionForward`) (`self.FLOOR_BOX_EXTENT`) true)
      (`BoxComponent.SetBoxExtent` (`self.FloorCollisionBackward`) (`self.FLOOR_BOX_EXTENT`) true)
      (`BoxComponent.SetBoxExtent` (`self.FloorCollisionLeft`) (`self.FLOOR_BOX_EXTENT`) true)
      (`BoxComponent.SetBoxExtent` (`self.FloorCollisionRight`) (`self.FLOOR_BOX_EXTENT`) true)
      (`self.SetCollisionResponseToChannel` (`self.FloorCollisionForward`) "ECC_GameTraceChannel6" "ECR_Block")
      (`self.SetCollisionResponseToChannel` (`self.FloorCollisionBackward`) "ECC_GameTraceChannel6" "ECR_Block")
      (`self.SetCollisionResponseToChannel` (`self.FloorCollisionLeft`) "ECC_GameTraceChannel6" "ECR_Block")
      (`self.SetCollisionResponseToChannel` (`self.FloorCollisionRight`) "ECC_GameTraceChannel6" "ECR_Block")
      (`self.SetCollisionResponseToChannel` (`self.FloorCollisionForward`) "ECC_GameTraceChannel7" "ECR_Block")
      (`self.SetCollisionResponseToChannel` (`self.FloorCollisionBackward`) "ECC_GameTraceChannel7" "ECR_Block")
      (`self.SetCollisionResponseToChannel` (`self.FloorCollisionLeft`) "ECC_GameTraceChannel7" "ECR_Block")
      (`self.SetCollisionResponseToChannel` (`self.FloorCollisionRight`) "ECC_GameTraceChannel7" "ECR_Block"))
    (:`then_5`
      ;[1 1 1] Wall Forward
      (bind _returnvalue_5 (`self.CreateCollision` (`self.WALL_LOCATION_FORWARD`) (`self.WALL_ROTATION_FORWARD`)))
      (bind _output_get_5 (set `self.WallCollisionForward` _returnvalue_5))
      (`self.CreateDebugCollision` _output_get_5 "Forward"))
    (:`then_6`
      ;[1 1 1] Wall Backward
      (bind _returnvalue_6 (`self.CreateCollision` (`self.WALL_LOCATION_BACKWARD`) (`self.WALL_ROTATION_BACKWARD`)))
      (bind _output_get_6 (set `self.WallCollisionBackward` _returnvalue_6))
      (`self.CreateDebugCollision` _output_get_6 "Backward"))
    (:`then_7`
      ;[1 1 1] Wall Left
      (bind _returnvalue_7 (`self.CreateCollision` (`self.WALL_LOCATION_LEFT`) (`self.WALL_ROTATION_LEFT`)))
      (bind _output_get_7 (set `self.WallCollisionLeft` _returnvalue_7))
      (`self.CreateDebugCollision` _output_get_7 "Left"))
    (:`then_8`
      ;[1 1 1] Wall Right
      (bind _returnvalue_8 (`self.CreateCollision` (`self.WALL_LOCATION_RIGHT`) (`self.WALL_ROTATION_RIGHT`)))
      (bind _output_get_8 (set `self.WallCollisionRight` _returnvalue_8))
      (`self.CreateDebugCollision` _output_get_8 "Right"))
    (:`then_9`
      ;[1 1 1] Wall Default Settings
      (`BoxComponent.SetBoxExtent` (`self.WallCollisionForward`) (`self.WALL_BOX_EXTENT`) true)
      (`BoxComponent.SetBoxExtent` (`self.WallCollisionBackward`) (`self.WALL_BOX_EXTENT`) true)
      (`BoxComponent.SetBoxExtent` (`self.WallCollisionLeft`) (`self.WALL_BOX_EXTENT`) true)
      (`BoxComponent.SetBoxExtent` (`self.WallCollisionRight`) (`self.WALL_BOX_EXTENT`) true)
      (`self.SetCollisionResponseToChannel` (`self.WallCollisionForward`) "ECC_GameTraceChannel4" "ECR_Block")
      (`self.SetCollisionResponseToChannel` (`self.WallCollisionBackward`) "ECC_GameTraceChannel4" "ECR_Block")
      (`self.SetCollisionResponseToChannel` (`self.WallCollisionLeft`) "ECC_GameTraceChannel4" "ECR_Block")
      (`self.SetCollisionResponseToChannel` (`self.WallCollisionRight`) "ECC_GameTraceChannel4" "ECR_Block"))
    (:`then_10`
      ;[1 1 1] Ladder
      (bind _returnvalue_9 (`self.CreateCollision` (`self.LADDER_LOCATION`) (`self.LADDER_ROTATION`)))
      (bind _output_get_9 (set `self.LadderCollision` _returnvalue_9))
      (`self.CreateDebugCollision` _output_get_9 "Ladder"))
    (:`then_11`
      ;[1 1 1] Ladder Default Settings
      (`BoxComponent.SetBoxExtent` (`self.LadderCollision`) (`self.LADDER_BOX_EXTENT`) true)
      (`self.SetCollisionResponseToChannel` (`self.LadderCollision`) "ECC_GameTraceChannel5" "ECR_Block"))))