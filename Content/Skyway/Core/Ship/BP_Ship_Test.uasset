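; BP_Ship_Test is a test ship Blueprint that adds a weather direction indicator and player respawning to its parent's behavior.
; WeatherDirectionArrow points along the weather direction, set at BeginPlay and updated on each weather change after the parent handles it.
; When the first player's character begins overlapping RespawnCollision, it teleports to the RespawnLocation component's world position without a sweep.
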(event `self.ReceiveBeginPlay`
  (`parent.ReceiveBeginPlay`)
  (`SceneComponent.K2_SetWorldRotation` (`self.WeatherDirectionArrow`) (`KismetMathLibrary.Conv_VectorToRotator` (`self.WeatherDirection`)) false false))

(event `self.RespawnCollision.OnComponentBeginOverlap`
  (params (OverlappedComponent :type "PrimitiveComponent Object Reference") (OtherActor :type "Actor Object Reference") (OtherComp :type "PrimitiveComponent Object Reference") (OtherBodyIndex :type Integer) (bFromSweep :type Boolean) (SweepResult :type "HitResult Structure (by ref)"))
  (if (== OtherActor (`GameplayStatics.GetPlayerCharacter` 0))
    (`self.K2_SetActorLocation` OtherActor (`SceneComponent.K2_GetComponentLocation` (`self.RespawnLocation`)) false true)))

(event `self.OnWeatherChange`
  (params (Speed :type "Float (double-precision)") (Direction :type "Vector Structure"))
  (`parent.OnWeatherChange` Speed Direction)
  (`SceneComponent.K2_SetWorldRotation` (`self.WeatherDirectionArrow`) (`KismetMathLibrary.Conv_VectorToRotator` Direction) false false))

(fn `UserConstructionScript`
  (`parent.UserConstructionScript`))