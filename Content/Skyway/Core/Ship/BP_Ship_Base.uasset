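; Base ship actor that is assembled at runtime from building components and tracks the weather's wind values.
; BeginPlay chains default foundations from DT_Buildables, with Build snapping pieces to connection boxes and disabling their collision.
; BP_Weather supplies speed and direction, which each tick feed ProjectileMovement's max speed and the resource spawner's direction.
; Move is an empty stub, with its manual location update left disconnected.
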(event `self.ReceiveBeginPlay`
  (`self.SpawnDefaultFoundation`)
  (bind _returnvalue (`GameplayStatics.GetActorOfClass` "/Game/Skyway/Core/Weather/BP_Weather.BP_Weather_C"))
  (set `self.WeatherSpeed` (`/Game/Skyway/Core/Weather/BP_Weather.Speed` _returnvalue))
  (set `self.WeatherDirection` (`/Game/Skyway/Core/Weather/BP_Weather.Direction` _returnvalue))
  (add `/Game/Skyway/Core/Weather/BP_Weather.OnWeatherChange` _returnvalue (`|CreateDelegate` :!event `OnWeatherChange`)))

(event `self.ReceiveTick`
  (params (DeltaSeconds :type "Float (single-precision)"))
  (`self.CalculateDirectionAndSpeed`)
  (`self.Move`)
  (`/Game/Skyway/Core/Building/Resources/Spawn/AC_SpawnResources.SetSpawnDirection` (`self.SpawnResources`) (`self.Direction`)))

(event `OnWeatherChange`
  (params (Speed :type "Float (double-precision)") (Direction :type "Vector Structure"))
  (set `self.WeatherSpeed` Speed)
  (set `self.WeatherDirection` Direction))

(event `self.DestroyBuilding`
  (params (Building :type "ActorComponent Object Reference"))
  (`ActorComponent.K2_DestroyComponent` Building))

(fn `Build`
  (params (BuildingInfo :type "/Game/Skyway/Core/Building/S_Buildables Structure") (HitBuildingComponent :type "SceneComponent Object Reference"))
  (locals (L_Building :type "/Game/Skyway/Core/Building/AC_Building_Base Object Reference"))
  (bind _hitbuildingcomponent (`local.HitBuildingComponent`))
  (bind _returnvalue (`|AddComponentByClass` (`.Class_13_A274FEF740D5D4E629676FA687CC24EA` (break `/Game/Skyway/Core/Building/S_Buildables` (`local.BuildingInfo`))) false (`/Game/Skyway/Core/Engine/MLBP_Defaults.DEFAULT`)))
  (set `local.L_Building` _returnvalue)
  (`KismetArrayLibrary.Array_Add` (`self.Buildings`) (`local.L_Building`))
  (`StaticMeshComponent.SetStaticMesh` (`local.L_Building`) (`.Mesh_2_8896AF7342135A205A3D19A098B64417` (break `/Game/Skyway/Core/Building/S_Buildables` (`local.BuildingInfo`))))
  (`/Engine/EditorBlueprintResources/StandardMacros.IsValid` _hitbuildingcomponent
    (:`Is Valid`
      (set `self.BuildingTransform` (`KismetMathLibrary.MakeTransform` (`SceneComponent.K2_GetComponentLocation` _hitbuildingcomponent) (`SceneComponent.K2_GetComponentRotation` _hitbuildingcomponent) (`/Game/Skyway/Core/Engine/MLBP_Defaults.DEFAULT_SCALE`)))
      (`SceneComponent.K2_SetWorldTransform` (`local.L_Building`) (`self.BuildingTransform`) false false)
      (bind _asbox_collision (cast `BoxComponent` (`local.HitBuildingComponent`)))
      (`PrimitiveComponent.SetCollisionEnabled` _asbox_collision "NoCollision"))))

(fn `CalculateDirectionAndSpeed`
  (set `self.Direction` (`self.WeatherDirection`))
  (bind _output_get (set `self.Speed` (`self.WeatherSpeed`)))
  (set `ProjectileMovementComponent.MaxSpeed` _output_get (`self.ProjectileMovement`)))

(fn `Move`)

(fn `SpawnDefaultFoundation`
  (locals (L_BuildingInfo :type "/Game/Skyway/Core/Building/S_Buildables Structure"))
  (bind _returnvalue (`|GetDataTableRow` "/Game/Skyway/Core/Building/DT_Buildables.DT_Buildables" "Fundation")
    (:`then`
      (set `local.L_BuildingInfo` _returnvalue)
      (for _index (range (`self.DefaultFoundationCount`))
        (if (!= _index 0)
          (bind _boxes (message `/Game/Skyway/Core/Building/BPI_Build.ReturnBoxes` (`|GetArrayItem` (`self.Buildings`) (- _index 1))))
          (`self.Build` (`local.L_BuildingInfo`) (`|GetArrayItem` _boxes 1))
          (else
            (`self.Build` (`local.L_BuildingInfo`))))))))

(fn `UserConstructionScript`)